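; BP_ZombieSpawner runs endless zombie waves, spawning BP_Zombie at its Arrow component.
; After a timed countdown, Spawn re-calls itself with random delays until the zombie count exceeds CurrentWave plus MaxAmountInWorld, so waves grow each round.
; A single timer handle then switches to polling IsWaveCleared, which increments the wave and restarts the countdown once no zombies remain.
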(event Custom|Spawn
  (Utilities|Time|ClearandInvalidateTimerbyHandle (Variables|Default|GetSpawner%20Timer))
  (Development|PrintString (Utilities|String|ToString(Text) (Utilities|Text|FormatText "Incoming Zombie Wave {Wave}" (Variables|Default|GetCurrentWave))))
  (bind _returnvalue (CallFunction|IsTooMuchZombies))
  (if _returnvalue
    (bind _returnvalue_2 (Utilities|Time|SetTimerbyEvent (delegate Custom|Is%20Wave%20Cleared) 3.0 true))
    (Variables|Default|SetSpawner%20Timer _returnvalue_2)
    (else
      (Game|SpawnActorfromClass "/Game/BP_Zombie.BP_Zombie_C" (Transformation|GetWorldTransform (Variables|Default|GetArrow)) "AlwaysSpawn" 0 0)
      (Utilities|FlowControl|Delay (Math|Random|RandomFloatinRange 1.0 2.0))
      (CallFunction|Spawn))))

(event Custom|Is%20Wave%20Cleared
  ;[1 1 1] Wave survived - start new countdown
  (if (== (CallFunction|CountZombies) 0)
    (Development|PrintString "Wave survived!" true true "(R=0.000000,G=1.000000,B=0.099035,A=1.000000)" 5.0)
    (Math|Integer|IncrementInt (Variables|Default|GetCurrentWave)
      (:%20%20
        (Utilities|Time|ClearandInvalidateTimerbyHandle (Variables|Default|GetSpawner%20Timer))
        (bind _returnvalue (Utilities|Time|SetTimerbyEvent (delegate Custom|Spawn) (Variables|Default|GetSpawnTimer) true))
        (Variables|Default|SetSpawner%20Timer _returnvalue)))))

(event EventBeginPlay
  (bind _returnvalue (Utilities|Time|SetTimerbyEvent (delegate Custom|Spawn) (Variables|Default|GetSpawnTimer) true))
  (Variables|Default|SetSpawner%20Timer _returnvalue))

(fn ConstructionScript)

(fn IsTooMuchZombies
  (return (> (CallFunction|CountZombies) (+ (Variables|Default|GetCurrentWave) (Variables|Default|GetMaxAmountInWorld)))))