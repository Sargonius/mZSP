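; Blueprint function library of global helpers for a zombie survival game with a camp.
; It finds the first camp actor, counts live zombie actors, and reads survival time from BP_GameMode_mzsp.
; Game speed functions store the value on that game mode and apply it as global time dilation.
; Stepping up or down clamps the speed between zero and three, while the direct setter does not clamp.
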(fn GetCamp
  (bind _outactors (Actor|GetAllActorsOfClass (Game|GetGameState) "/Game/BP_Camp.BP_Camp_C"))
  (return (Utilities|Array|Get(acopy) _outactors)))

(fn GetGameSpeed
  (bind _asbp_game_mode_mzsp (Utilities|Casting|CastToBP_GameMode_mzsp (Game|GetGameMode)))
  (return (Variables|/Game/BP_GameMode_mzsp.BP_GameMode_mzsp_C|GetGameSpeed _asbp_game_mode_mzsp)))

(fn CountZombies
  (bind _outactors (Actor|GetAllActorsOfClass (LocalVariables|Get__WorldContext) "/Game/BP_Zombie.BP_Zombie_C"))
  (return (Utilities|Array|Length _outactors)))

(fn IncreaseGameSpeed
  (bind _asbp_game_mode_mzsp (Utilities|Casting|CastToBP_GameMode_mzsp (Game|GetGameMode)))
  (bind _output_get (Variables|/Game/BP_GameMode_mzsp.BP_GameMode_mzsp_C|SetGameSpeed _asbp_game_mode_mzsp (Math|Float|Clamp(Float) (+ (Variables|/Game/BP_GameMode_mzsp.BP_GameMode_mzsp_C|GetGameSpeed _asbp_game_mode_mzsp) 1.0) 0.0 3.0)))
  (Utilities|Time|SetGlobalTimeDilation 0 _output_get)
  (return))

(fn DecreaseGameSpeed
  (bind _asbp_game_mode_mzsp (Utilities|Casting|CastToBP_GameMode_mzsp (Game|GetGameMode)))
  (bind _output_get (Variables|/Game/BP_GameMode_mzsp.BP_GameMode_mzsp_C|SetGameSpeed _asbp_game_mode_mzsp (Math|Float|Clamp(Float) (+ (Variables|/Game/BP_GameMode_mzsp.BP_GameMode_mzsp_C|GetGameSpeed _asbp_game_mode_mzsp) -1.0) 0.0 3.0)))
  (Utilities|Time|SetGlobalTimeDilation 0 _output_get)
  (return))

(fn SetGameSpeed
  (params (GameSpeed :type Float%20%28single-precision%29))
  (bind _asbp_game_mode_mzsp (Utilities|Casting|CastToBP_GameMode_mzsp (Game|GetGameMode)))
  (bind _output_get (Variables|/Game/BP_GameMode_mzsp.BP_GameMode_mzsp_C|SetGameSpeed _asbp_game_mode_mzsp GameSpeed))
  (Utilities|Time|SetGlobalTimeDilation 0 _output_get)
  (return))

(fn GetSurvivalTime
  (bind _asbp_game_mode_mzsp (Utilities|Casting|CastToBP_GameMode_mzsp (Game|GetGameMode)))
  (return (Variables|/Game/BP_GameMode_mzsp.BP_GameMode_mzsp_C|GetSurvivalTime _asbp_game_mode_mzsp)))