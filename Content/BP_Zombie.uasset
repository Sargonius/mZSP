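; Zombie AI that wanders the map and attacks damageable actors, driven by an enum state machine on a looping one-second timer.
; It moves to random reachable points around the world origin until its Perception overlap finds a BPI_Damageable target.
; Attacking stops movement and starts a self-repeating loop that faces the target, deals damage and plays a timeline body lunge.
; When the target becomes invalid, it resumes wandering.
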(event OnComponentBeginOverlap(Perception)
  (params (OverlappedComponent :type Primitive%20Component%20Object%20Reference) (OtherActor :type Actor%20Object%20Reference) (OtherComp :type Primitive%20Component%20Object%20Reference) (OtherBodyIndex :type Integer) (bFromSweep :type Boolean) (SweepResult :type Hit%20Result%20Structure%20%28by%20ref%29))
  (Utilities|IsValid (Variables|Default|GetTarget%20To%20Attack)
    (:Is%20Not%20Valid
      (if (Utilities|DoesObjectImplementInterface OtherActor "/Game/BPI_Damageable.BPI_Damageable_C")
        (Variables|Default|SetTarget%20To%20Attack OtherActor)))))

(event Custom|Play%20Attack%20Animation
  ;[1 1 1] Attack Animation
  (bind _attack_x (Timeline|Timeline_0 PlayFromStart)
    (:Update
      (Transformation|SetRelativeLocation (Variables|Default|GetBody) (Math|Vector|MakeVector _attack_x 0.0 0.0) false false))
    (:Finished
      (CallFunction|CombatLoop))))

(event Custom|Combat%20Loop
  (bind _target_to_attack (Variables|Default|GetTarget%20To%20Attack))
  (bind _returnvalue (Transformation|GetActorLocation _target_to_attack))
  (Utilities|IsValid _target_to_attack
    (:Is%20Valid
      (Transformation|SetActorRotation (Math|Rotator|MakeRotator 0.0 0.0 (.yaw (Math|Rotator|FindLookatRotation (Transformation|GetActorLocation) _returnvalue))))
      (Variables|Default|SetTarget%20Location _returnvalue)
      (CallFunction|PlayAttackAnimation)
      (Class|BPIDamageable|TakeDamage(Message) (Variables|Default|GetTarget%20To%20Attack) (Variables|Default|GetDamage)))
    (:Is%20Not%20Valid
      (Variables|Default|SetState "NewEnumerator0")
      (CallFunction|CombatEnded))))

(event Custom|Logic%20Loop
  (switch Utilities|FlowControl|Switch|SwitchonFZombieStates (Variables|Default|GetState)
    (:NewEnumerator0
      (CallFunction|FindNewTarget))
    (:NewEnumerator1
      (AI|Navigation|SimpleMovetoLocation (AI|GetAIController self) (Variables|Default|GetTarget%20Location))
      (Utilities|IsValid (Variables|Default|GetTarget%20To%20Attack)
        (:Is%20Valid
          (Variables|Default|SetState "NewEnumerator2"))
        (:Is%20Not%20Valid
          (if (<= (.PathLength (Class|NavigationSystem|GetPathLength (Transformation|GetActorLocation) (Variables|Default|GetTarget%20Location))) 5e+01)
            (Variables|Default|SetState "NewEnumerator0")))))
    (:NewEnumerator2
      (Utilities|FlowControl|DoOnce false
        (:Completed
          (CallFunction|CombatLoop)
          (Components|Movement|StopMovementImmediately (Variables|Character|GetCharacterMovement)))))))

(event Custom|Combat%20Ended
  (Utilities|FlowControl|DoOnce false) ; enters at Reset
)

(event EventTick
  (params (DeltaSeconds :type Float%20%28single-precision%29))
  ;[1 1 1] Debug State
)

(event EventBeginPlay
  ;[1 1 1] Start Logic Loop
  (Utilities|Time|SetTimerbyEvent (delegate Custom|Logic%20Loop) 1.0 true))

(fn ConstructionScript)

(fn UpdateDebugStateText
  (Rendering|Components|TextRender|SetText (Variables|Default|GetCurrentState) (Utilities|Text|ToText(String) (Utilities|String|EnumtoString (Variables|Default|GetState)))))

(fn FindNewTarget
  (Variables|Default|SetTarget%20Location (.RandomLocation (AI|Navigation|GetRandomReachablePointinRadius (Math|Vector|MakeVector 0.0 0.0 0.0) (Variables|Default|GetRadius%20For%20Target%20Search))))
  (Variables|Default|SetState "NewEnumerator1"))