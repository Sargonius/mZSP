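; Clickable building that grows a cluster by spawning another BP_Building in a random free neighboring slot, sometimes adding a BP_Decoration when FreeSlots equals one.
; Four side colliders act as slots, switching their component tags between Free and NotFree on overlap, and placement picks among the Free-tagged ones.
; Spawned actors get random yaw, and buildings also get random height.
; Tick draws debug boxes on free slots and updates the free-slot count text.
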(event OnClicked(MainBuilding)
  (params (TouchedComponent :type Primitive%20Component%20Object%20Reference) (ButtonPressed :type Key%20Structure))
  (CallFunction|GetFreeSlotandBuildinIt "BP_Building_C")
  (if (== (Variables|Default|GetFree%20Slots) 1)
    (if (> (Math|Random|RandomFloat) 0.6)
      (CallFunction|GetFreeSlotandBuildinIt "/Game/BP_Decoration.BP_Decoration_C"))))

(event Custom|Build%20Object%20in%20Slot
  (params (Slot :type Box%20Component%20Object%20Reference) (Object :type Actor%20Class%20Reference))
  (bind _returnvalue (Game|SpawnActorfromClass Object (Transformation|GetWorldTransform Slot) "Undefined" 0 0))
  (Math|Integer|DecrementInt (Variables|Default|GetFree%20Slots)
    (:%20%20
      (Transformation|SetActorRotation _returnvalue (Math|Rotator|MakeRotator 0.0 0.0 (Math|Random|RandomFloatinRange 0.0 3.6e+02)))
      (bind _asbp_building (Utilities|Casting|CastToBP_Building _returnvalue))
      (Transformation|SetWorldScale3D (Variables|BP_Building_C|GetMainBuilding _asbp_building) (Math|Vector|MakeVector 1.0 1.0 (Math|Random|RandomFloatinRange 0.5 1.6))))))

(event EventBeginPlay)

(event Collision|EventActorBeginOverlap
  (params (OtherActor :type Actor%20Object%20Reference)))

(event EventTick
  (params (DeltaSeconds :type Float%20%28single-precision%29))
  (CallFunction|DrawDebugSlotInfo (Variables|Default|GetLeft%20Collider))
  (CallFunction|DrawDebugSlotInfo (Variables|Default|GetUp%20Collider))
  (CallFunction|DrawDebugSlotInfo (Variables|Default|GetRight%20Collider))
  (CallFunction|DrawDebugSlotInfo (Variables|Default|GetDown%20Collider))
  (Rendering|Components|TextRender|SetText (Variables|Default|GetFreeSlots) (Utilities|Text|ToText(Integer) (.Free%20Slots (Slots|CountFreeSlots)))))

(event OnComponentBeginOverlap(LeftCollider)
  (params (OverlappedComponent :type Primitive%20Component%20Object%20Reference) (OtherActor :type Actor%20Object%20Reference) (OtherComp :type Primitive%20Component%20Object%20Reference) (OtherBodyIndex :type Integer) (bFromSweep :type Boolean) (SweepResult :type Hit%20Result%20Structure%20%28by%20ref%29))
  ;[1 1 1] Overlapped - NotFree
  (Slots|UpdateSlotState OverlappedComponent "NotFree"))

(event OnComponentBeginOverlap(UpCollider)
  (params (OverlappedComponent :type Primitive%20Component%20Object%20Reference) (OtherActor :type Actor%20Object%20Reference) (OtherComp :type Primitive%20Component%20Object%20Reference) (OtherBodyIndex :type Integer) (bFromSweep :type Boolean) (SweepResult :type Hit%20Result%20Structure%20%28by%20ref%29))
  ;[1 1 1] Overlapped - NotFree
  (Slots|UpdateSlotState OverlappedComponent "NotFree"))

(event OnComponentEndOverlap(DownCollider)
  (params (OverlappedComponent :type Primitive%20Component%20Object%20Reference) (OtherActor :type Actor%20Object%20Reference) (OtherComp :type Primitive%20Component%20Object%20Reference) (OtherBodyIndex :type Integer))
  ;[1 1 1] Overlap end - Free
  (Slots|UpdateSlotState OverlappedComponent "Free"))

(event OnComponentBeginOverlap(DownCollider)
  (params (OverlappedComponent :type Primitive%20Component%20Object%20Reference) (OtherActor :type Actor%20Object%20Reference) (OtherComp :type Primitive%20Component%20Object%20Reference) (OtherBodyIndex :type Integer) (bFromSweep :type Boolean) (SweepResult :type Hit%20Result%20Structure%20%28by%20ref%29))
  ;[1 1 1] Overlapped - NotFree
  (Slots|UpdateSlotState OverlappedComponent "NotFree"))

(event OnComponentBeginOverlap(RightCollider)
  (params (OverlappedComponent :type Primitive%20Component%20Object%20Reference) (OtherActor :type Actor%20Object%20Reference) (OtherComp :type Primitive%20Component%20Object%20Reference) (OtherBodyIndex :type Integer) (bFromSweep :type Boolean) (SweepResult :type Hit%20Result%20Structure%20%28by%20ref%29))
  ;[1 1 1] Overlapped - NotFree
  (Slots|UpdateSlotState OverlappedComponent "NotFree"))

(event OnComponentEndOverlap(LeftCollider)
  (params (OverlappedComponent :type Primitive%20Component%20Object%20Reference) (OtherActor :type Actor%20Object%20Reference) (OtherComp :type Primitive%20Component%20Object%20Reference) (OtherBodyIndex :type Integer))
  ;[1 1 1] Overlap end - Free
  (Slots|UpdateSlotState OverlappedComponent "Free"))

(event OnComponentEndOverlap(UpCollider)
  (params (OverlappedComponent :type Primitive%20Component%20Object%20Reference) (OtherActor :type Actor%20Object%20Reference) (OtherComp :type Primitive%20Component%20Object%20Reference) (OtherBodyIndex :type Integer))
  ;[1 1 1] Overlap end - Free
  (Slots|UpdateSlotState OverlappedComponent "Free"))

(event OnComponentEndOverlap(RightCollider)
  (params (OverlappedComponent :type Primitive%20Component%20Object%20Reference) (OtherActor :type Actor%20Object%20Reference) (OtherComp :type Primitive%20Component%20Object%20Reference) (OtherBodyIndex :type Integer))
  ;[1 1 1] Overlap end - Free
  (Slots|UpdateSlotState OverlappedComponent "Free"))

(fn ConstructionScript)

(fn CountFreeSlots
  (bind _output_get (Variables|Default|SetFree%20Slots (Utilities|Array|Length (Actor|GetComponentsbyTag "/Script/Engine.BoxComponent" "Free"))))
  (Development|PrintString (Utilities|String|ToString(Text) (Utilities|Text|FormatText "Free slots: {count}" _output_get)))
  (return _output_get (> _output_get 0)))

(fn GetFreeSlot
  (bind _returnvalue (Actor|GetComponentsbyTag "/Script/Engine.BoxComponent" "Free"))
  (bind _hasfreeslot (Slots|CountFreeSlots))
  (if _hasfreeslot
    (return _hasfreeslot (Utilities|Array|Get(acopy) _returnvalue (Math|Random|RandomIntegerinRange 0 (- (Utilities|Array|Length _returnvalue) 1))))
    (else
      (return _hasfreeslot 0))))

(fn GetSlotState
  (params (Slot :type Object%20Object%20Reference) (Tag%20Array :type Array%20of%20Names))
  (Development|PrintString (Utilities|String|ToString(Text) (Utilities|Text|FormatText "Slot {name} {state}" (Utilities|Text|ToText(String) (Utilities|GetDisplayName Slot)) (Utilities|Text|ToText(Name) (Utilities|Array|Get(acopy) Tag%20Array))))))

(fn UpdateSlotState
  (params (Slot :type Actor%20Component%20Object%20Reference) (State :type Name))
  (bind _output_get (Variables|/Script/Engine.ActorComponent|SetComponentTags Slot (Utilities|Array|MakeArray State)))
  (Slots|GetSlotState Slot _output_get))

(fn GetFreeSlotandBuildinIt
  (params (Object :type Actor%20Class%20Reference))
  (bind (_hasfreeslot _slot) (Slots|GetFreeSlot))
  (if _hasfreeslot
    (CallFunction|BuildObjectinSlot _slot Object)))

(fn DrawDebugSlotInfo
  (params (Slot :type Scene%20Component%20Object%20Reference))
  (if (Components|ComponentHasTag Slot "Free")
    (Rendering|Debug|DrawDebugBox (Transformation|GetWorldLocation Slot) "60.000000,60.000000,60.000000" (Utilities|Struct|MakeLinearColor 0.0 255.0 0.0 1.0) "0, 0, 0" 0.0 1.0)))