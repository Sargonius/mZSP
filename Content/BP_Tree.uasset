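; BP_Tree is a tree actor that randomizes its look when play begins, so placed copies differ from one another.
; On BeginPlay it sets random Green and Yellow scalar parameters on the static mesh's materials to vary color.
; It then applies a random non-uniform scale, with a wider range on height, and a random yaw over a full turn.
; The construction script is empty, so the variation appears only at runtime.
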(event EventBeginPlay
  (Rendering|Material|SetScalarParameterValueonMaterials (Variables|Debug|GetStaticMeshComponent) "Green" (Math|Random|RandomFloatinRange 0.0 0.4))
  (Rendering|Material|SetScalarParameterValueonMaterials (Variables|Debug|GetStaticMeshComponent) "Yellow" (Math|Random|RandomFloatinRange 0.0 0.4))
  (Transformation|SetActorScale3D (Math|Vector|MakeVector (Math|Random|RandomFloatinRange 0.85 1.15) (Math|Random|RandomFloatinRange 0.85 1.15) (Math|Random|RandomFloatinRange 0.7 1.25)))
  (Transformation|SetActorRotation (Math|Rotator|MakeRotator 0.0 0.0 (Math|Random|RandomFloatinRange 0.0 3.6e+02))))

(event Collision|EventActorBeginOverlap
  (params (OtherActor :type Actor%20Object%20Reference)))

(event EventTick
  (params (DeltaSeconds :type Float%20%28single-precision%29)))

(fn ConstructionScript)