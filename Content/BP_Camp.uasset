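; BP_Camp is a camp actor that stores Food and Materials and drives settlement expansion.
; UnloadResources splits incoming resources evenly between the two stores.
; ExpandCamp spawns a BP_Building at the camp's transform if none exist in the level.
; Otherwise it calls TryToBuildHouse on each building in turn, breaking the loop on the first success or report of no materials.
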(event Custom|Expand%20Camp
  (bind _outactors (Actor|GetAllActorsOfClass "/Game/BP_Building.BP_Building_C"))
  (if (== (Utilities|Array|Length _outactors) 0)
    ;[1 1 1] No Buildings Left - spawn one
    (Game|SpawnActorfromClass "/Game/BP_Building.BP_Building_C" (Transformation|GetActorTransform) "Undefined" 0 0)
    (else
      (bind _array_element (Utilities|Array|ForEachLoopwithBreak _outactors)
        (:LoopBody
          (bind (_isbuild _nomaterials) (Default|TrytoBuildHouse _array_element))
          (if _isbuild
            (CallFunction|BreakBuildCycle)
            (elif _nomaterials
              (CallFunction|BreakBuildCycle))))))))

(event Custom|Break%20Build%20Cycle
  (Utilities|Array|ForEachLoopwithBreak (stale Custom|Expand%20Camp _outactors)) ; enters at Break
)

(event Custom|Unload%20Resources
  (params (Found%20Resources :type Float%20%28single-precision%29))
  (bind _returnvalue (/ Found%20Resources 2.0))
  (Variables|Default|SetFood (+ (Variables|Default|GetFood) _returnvalue))
  (Variables|Default|SetMaterials (+ (Variables|Default|GetMaterials) _returnvalue)))

(fn ConstructionScript)