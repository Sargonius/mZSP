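; Raid building actor that can be looted, damaged and extended with neighboring objects.
; Four side colliders tag themselves Free or NotFree on overlaps, and build functions spawn into a random free slot with random yaw, randomizing height for buildings.
; Looting sets a flag that clears after a random delay, shown as text each tick.
; A looping timer tints the mesh by health, and zero health triggers an explosion and destroys it.
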(event Custom|DebugBuild
  (CallFunction|GetFreeSlotandBuildinIt "BP_RaidBuilding_C"))

(event Custom|Update%20Building%20Health
  (bind _health (Variables|Default|GetHealth))
  (bind _returnvalue (Math|Float|MapRangeClamped _health 0.0 1e+02 0.0 1.0))
  (Rendering|Material|SetVectorParameterValueonMaterials (Variables|Default|GetMainBuilding) "Color" (Math|Vector|MakeVector 1.0 _returnvalue _returnvalue)))

(event Custom|Looted
  (Variables|Default|SetisLooted true)
  (Utilities|FlowControl|Delay (Math|Random|RandomFloatinRange 15.0 3e+01))
  (Variables|Default|SetisLooted false))

(event Custom|Build%20Object%20in%20Slot
  (params (Slot :type Box%20Component%20Object%20Reference) (Object :type Actor%20Class%20Reference))
  (bind _returnvalue (Game|SpawnActorfromClass Object (Transformation|GetWorldTransform Slot) "Undefined" 0 0))
  (Math|Integer|DecrementInt (Variables|Default|GetFree%20Slots)
    (:%20%20
      (Transformation|SetActorRotation _returnvalue (Math|Rotator|MakeRotator 0.0 0.0 (Math|Random|RandomFloatinRange 0.0 3.6e+02)))
      (bind _asbp_raid_building (Utilities|Casting|CastToBP_RaidBuilding _returnvalue))
      (Transformation|SetWorldScale3D (Variables|BP_RaidBuilding_C|GetMainBuilding _asbp_raid_building) (Math|Vector|MakeVector 1.0 1.0 (Math|Random|RandomFloatinRange 1.5 3.0))))))

(event EventTick
  (params (DeltaSeconds :type Float%20%28single-precision%29))
  (Rendering|Components|TextRender|SetText (Variables|Default|GetFreeSlots) (Utilities|Text|ToText(Boolean) (Variables|Default|GetisLooted))))

(event EventTakeDamage
  (params (Damage :type Float%20%28single-precision%29))
  (Variables|Default|SetHealth (Math|Float|Clamp(Float) (- (Variables|Default|GetHealth) Damage) 0.0 (Variables|Default|GetHealth)))
  (if (== (Variables|Default|GetHealth) 0.0)
    (Effects|SpawnEmitteratLocation "/Game/StarterContent/Particles/P_Explosion.P_Explosion" (Transformation|GetWorldLocation (Variables|Default|GetMainBuilding)))
    (Actor|DestroyActor)))

(event EventBeginPlay
  (Utilities|Time|SetTimerbyEvent (delegate Custom|Update%20Building%20Health) 1.0 true))

(event OnComponentBeginOverlap(LeftCollider)
  (params (OverlappedComponent :type Primitive%20Component%20Object%20Reference) (OtherActor :type Actor%20Object%20Reference) (OtherComp :type Primitive%20Component%20Object%20Reference) (OtherBodyIndex :type Integer) (bFromSweep :type Boolean) (SweepResult :type Hit%20Result%20Structure%20%28by%20ref%29))
  ;[1 1 1] Overlapped - NotFree
  (Slots|OccupySlot OverlappedComponent "NotFree"))

(event OnComponentBeginOverlap(UpCollider)
  (params (OverlappedComponent :type Primitive%20Component%20Object%20Reference) (OtherActor :type Actor%20Object%20Reference) (OtherComp :type Primitive%20Component%20Object%20Reference) (OtherBodyIndex :type Integer) (bFromSweep :type Boolean) (SweepResult :type Hit%20Result%20Structure%20%28by%20ref%29))
  ;[1 1 1] Overlapped - NotFree
  (Slots|OccupySlot OverlappedComponent "NotFree"))

(event OnComponentEndOverlap(DownCollider)
  (params (OverlappedComponent :type Primitive%20Component%20Object%20Reference) (OtherActor :type Actor%20Object%20Reference) (OtherComp :type Primitive%20Component%20Object%20Reference) (OtherBodyIndex :type Integer))
  ;[1 1 1] Overlap end - Free
  (Slots|FreeSlot OverlappedComponent "Free"))

(event OnComponentBeginOverlap(DownCollider)
  (params (OverlappedComponent :type Primitive%20Component%20Object%20Reference) (OtherActor :type Actor%20Object%20Reference) (OtherComp :type Primitive%20Component%20Object%20Reference) (OtherBodyIndex :type Integer) (bFromSweep :type Boolean) (SweepResult :type Hit%20Result%20Structure%20%28by%20ref%29))
  ;[1 1 1] Overlapped - NotFree
  (Slots|OccupySlot OverlappedComponent "NotFree"))

(event OnComponentBeginOverlap(RightCollider)
  (params (OverlappedComponent :type Primitive%20Component%20Object%20Reference) (OtherActor :type Actor%20Object%20Reference) (OtherComp :type Primitive%20Component%20Object%20Reference) (OtherBodyIndex :type Integer) (bFromSweep :type Boolean) (SweepResult :type Hit%20Result%20Structure%20%28by%20ref%29))
  ;[1 1 1] Overlapped - NotFree
  (Slots|OccupySlot OverlappedComponent "NotFree"))

(event OnComponentEndOverlap(LeftCollider)
  (params (OverlappedComponent :type Primitive%20Component%20Object%20Reference) (OtherActor :type Actor%20Object%20Reference) (OtherComp :type Primitive%20Component%20Object%20Reference) (OtherBodyIndex :type Integer))
  ;[1 1 1] Overlap end - Free
  (Slots|FreeSlot OverlappedComponent "Free"))

(event OnComponentEndOverlap(UpCollider)
  (params (OverlappedComponent :type Primitive%20Component%20Object%20Reference) (OtherActor :type Actor%20Object%20Reference) (OtherComp :type Primitive%20Component%20Object%20Reference) (OtherBodyIndex :type Integer))
  ;[1 1 1] Overlap end - Free
  (Slots|FreeSlot OverlappedComponent "Free"))

(event OnComponentEndOverlap(RightCollider)
  (params (OverlappedComponent :type Primitive%20Component%20Object%20Reference) (OtherActor :type Actor%20Object%20Reference) (OtherComp :type Primitive%20Component%20Object%20Reference) (OtherBodyIndex :type Integer))
  ;[1 1 1] Overlap end - Free
  (Slots|FreeSlot OverlappedComponent "Free"))

(fn ConstructionScript)

(fn CountFreeSlots
  (bind _output_get (Variables|Default|SetFree%20Slots (Utilities|Array|Length (Actor|GetComponentsbyTag "/Script/Engine.BoxComponent" "Free"))))
  (return _output_get (> _output_get 0)))

(fn GetFreeSlot
  (bind _returnvalue (Actor|GetComponentsbyTag "/Script/Engine.BoxComponent" "Free"))
  (bind _hasfreeslot (Slots|CountFreeSlots))
  (if _hasfreeslot
    (return _hasfreeslot (Utilities|Array|Get(acopy) _returnvalue (Math|Random|RandomIntegerinRange 0 (- (Utilities|Array|Length _returnvalue) 1))))
    (else
      (return _hasfreeslot 0))))

(fn GetSlotState
  (params (Slot :type Object%20Object%20Reference) (Tag%20Array :type Array%20of%20Names)))

(fn OccupySlot
  (params (Slot :type Actor%20Component%20Object%20Reference) (State :type Name))
  (bind _output_get (Variables|/Script/Engine.ActorComponent|SetComponentTags Slot (Utilities|Array|MakeArray State)))
  (Slots|GetSlotState Slot _output_get))

(fn GetFreeSlotandBuildinIt
  (params (Object :type Actor%20Class%20Reference))
  (bind (_hasfreeslot _slot) (Slots|GetFreeSlot))
  (if _hasfreeslot
    (CallFunction|BuildObjectinSlot _slot Object)))

(fn DrawDebugSlotInfo
  (params (Slot :type Scene%20Component%20Object%20Reference)))

(fn FreeSlot
  (params (Slot :type Actor%20Component%20Object%20Reference) (State :type Name))
  (bind _asbox_collision (Utilities|Casting|CastToBoxComponent Slot))
  (if (== (Utilities|Array|Length (Class|PrimitiveComponent|GetOverlappingComponents _asbox_collision)) 0)
    (bind _output_get (Variables|/Script/Engine.ActorComponent|SetComponentTags Slot (Utilities|Array|MakeArray State)))
    (Slots|GetSlotState Slot _output_get)))