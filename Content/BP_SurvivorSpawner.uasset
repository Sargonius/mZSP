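; BP_SurvivorSpawner adds new survivors to the camp over time, spawning BP_Survivor at its own transform.
; BeginPlay starts a looping timer whose interval is randomized once, between a few and several seconds.
; Each tick of that timer spawns only when the zombie count is zero and a free house is available, then prints a join message.
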(event Custom|Spawn%20Survivor
  (if (== (CallFunction|CountZombies) 0)
    (bind _bhasfreehouse (CallFunction|IsFreeHouseAvailable))
    (if _bhasfreehouse
      (Game|SpawnActorfromClass "/Game/BP_Survivor.BP_Survivor_C" (Transformation|GetActorTransform) "AlwaysSpawn" 0 0)
      (Development|PrintString "A Survivor joined your camp"))))

(event EventBeginPlay
  (Utilities|Time|SetTimerbyEvent (delegate Custom|Spawn%20Survivor) (Math|Random|RandomFloatinRange 5.0 15.0) true))

(event Collision|EventActorBeginOverlap
  (params (OtherActor :type Actor%20Object%20Reference)))

(event EventTick
  (params (DeltaSeconds :type Float%20%28single-precision%29)))

(fn ConstructionScript)