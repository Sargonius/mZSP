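; BP_Survivor is an autonomous survivor character that patrols, fights zombies and raids city buildings for camp resources.
; A timer-driven enum state machine picks targets, moves on navmesh and enters a Timeline-paced combat loop against enemies memorized by perception overlap.
; Survivors randomly join raids up to a population-based cap, returning when backpacks fill.
; Separate timers handle hunger and healing from camp stocks, overlaps repair buildings, and camera-facing text shows debug state.
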(event OnComponentBeginOverlap(Perception)
  (params (OverlappedComponent :type Primitive%20Component%20Object%20Reference) (OtherActor :type Actor%20Object%20Reference) (OtherComp :type Primitive%20Component%20Object%20Reference) (OtherBodyIndex :type Integer) (bFromSweep :type Boolean) (SweepResult :type Hit%20Result%20Structure%20%28by%20ref%29))
  ;[1 1 1] Spot Enemy, Memorize it and attack
  (bind _asbp_zombie (Utilities|Casting|CastToBP_Zombie OtherActor))
  (Utilities|Array|AddUnique (Variables|Combat|GetEnemies) 0)
  (Utilities|IsValid (Variables|Combat|GetTarget%20To%20Attack)
    (:Is%20Not%20Valid
      (Variables|Combat|SetTarget%20To%20Attack _asbp_zombie))))

(event OnComponentBeginOverlap(RepairRadius)
  (params (OverlappedComponent :type Primitive%20Component%20Object%20Reference) (OtherActor :type Actor%20Object%20Reference) (OtherComp :type Primitive%20Component%20Object%20Reference) (OtherBodyIndex :type Integer) (bFromSweep :type Boolean) (SweepResult :type Hit%20Result%20Structure%20%28by%20ref%29))
  (bind _camp (CallFunction|GetCamp))
  ;[1 1 1] Repair Buildings
  (bind _asbp_building (Utilities|Casting|CastToBP_Building OtherActor))
  (if (< (Variables|/Game/BP_Building.BP_Building_C|GetHealth _asbp_building) (Variables|/Game/BP_Building.BP_Building_C|GetMaxHealth _asbp_building))
    (if (> (Variables|/Game/BP_Camp.BP_Camp_C|GetMaterials _camp) 0.1)
      (Variables|/Game/BP_Camp.BP_Camp_C|SetMaterials _camp (- (Variables|/Game/BP_Camp.BP_Camp_C|GetMaterials _camp) 0.1))
      (Variables|/Game/BP_Building.BP_Building_C|SetHealth _asbp_building (Math|Float|Clamp(Float) (+ (Variables|/Game/BP_Building.BP_Building_C|GetHealth _asbp_building) (Math|Random|RandomFloatinRange 25.0 5e+01)) 0.0 (Variables|/Game/BP_Building.BP_Building_C|GetMaxHealth _asbp_building))))))

(event OnClicked(Body)
  (params (TouchedComponent :type Primitive%20Component%20Object%20Reference) (ButtonPressed :type Key%20Structure))
  ;[1 0 0] Debug
  (Rendering|Debug|DrawDebugSphere (Variables|Movement|GetTarget%20Location) 25.0 12 "(R=1.000000,G=0.037325,B=0.000000,A=1.000000)" 5.0 5.0))

(event OnComponentBeginOverlap(Body)
  (params (OverlappedComponent :type Primitive%20Component%20Object%20Reference) (OtherActor :type Actor%20Object%20Reference) (OtherComp :type Primitive%20Component%20Object%20Reference) (OtherBodyIndex :type Integer) (bFromSweep :type Boolean) (SweepResult :type Hit%20Result%20Structure%20%28by%20ref%29))
  ;[1 1 1] Unload Resources at camp after raid
  (if (and (> (Variables|Raid|GetFoundStuff) 0.0) (Actor|ActorHasTag OtherActor "Camp"))
    (Development|PrintString (Utilities|String|ToString(Text) (Utilities|Text|FormatText "Found stuff: {Stuff}" (Variables|Raid|GetFoundStuff))))))

(event Custom|Play%20Attack%20Animation
  ;[1 0 0] Attack Animation
  (bind _attack_x (Timeline|Timeline_0 PlayFromStart)
    (:Update
      (Transformation|SetRelativeLocation (Variables|Default|GetBody) (Math|Vector|MakeVector _attack_x 0.0 0.0) false false))
    (:Finished
      (CallFunction|CombatLoop))))

(event Custom|Go%20To%20Raid
  ;[1 1 1] Set Survivor in Raid Mode
  (Math|Float|IncrementFloat (Variables|/Game/BP_Camp.BP_Camp_C|GetSurvivors%20In%20Raid (CallFunction|GetCamp))
    (:%20%20
      (Variables|Raid|SetisInRaidMode true)
      (Development|SetHiddeninGame (Variables|Default|GetRaid%20Icon) false false)
      (Variables|Default|SetState "NewEnumerator0"))))

(event Custom|Combat%20Loop
  ;[1 0 0] Combat Loop
  (Variables|Combat|SetbIsInCombat true)
  (Utilities|IsValid (Variables|Combat|GetTarget%20To%20Attack)
    (:Is%20Valid
      (Combat|AttackTarget))
    (:Is%20Not%20Valid
      (Combat|IsCombatEndedandNoEnemiesLeft?))))

(event Custom|Logic%20Loop
  (switch Utilities|FlowControl|Switch|SwitchonFSurvivorStates (Variables|Default|GetState)
    (:NewEnumerator0
      (CallFunction|FindNewTarget))
    (:NewEnumerator1
      (CallFunction|MovingLogic))
    (:NewEnumerator2
      ;[1 0 0] Combat Loop
      (Utilities|FlowControl|DoOnce false
        (:Completed
          (CallFunction|CombatLoop)
          (Components|Movement|StopMovementImmediately (Variables|Character|GetCharacterMovement)))))))

(event Custom|Combat%20Ended
  ;[1 0 0] Combat Ended
  (Variables|Combat|SetbIsInCombat false)
  ;[1 0 0] Combat Loop
  (Utilities|FlowControl|DoOnce false) ; enters at Reset
)

(event Custom|Hunger%20Loop
  (CallFunction|Eat))

(event Custom|Needs%20Loop
  (Variables|Stats|SetHunger (+ (Variables|Stats|GetHunger) 0.2))
  (CallFunction|Heal))

(event Custom|Call%20Back%20From%20Raid
  ;[1 1 1] Set Survivor in Raid Mode
  (Math|Float|DecrementFloat (Variables|/Game/BP_Camp.BP_Camp_C|GetSurvivors%20In%20Raid (CallFunction|GetCamp))
    (:%20%20
      (Variables|Raid|SetisInRaidMode false)
      (Development|SetHiddeninGame (Variables|Default|GetRaid%20Icon) true false)
      (Variables|Default|SetState "NewEnumerator0"))))

(event EventTakeDamage
  (params (Damage :type Float%20%28single-precision%29))
  ;[1 0 0] Take Damage
  (Combat|OnTakeDamage Damage))

(event EventTick
  (params (DeltaSeconds :type Float%20%28single-precision%29))
  (CallFunction|UpdateDebugData))

(event EventBeginPlay
  ;[1 1 1] Start Logic Loop
  (Utilities|Time|SetTimerbyEvent (delegate Custom|Logic%20Loop) 0.2 true)
  (CallFunction|MakeRandomColor)
  (Utilities|Time|SetTimerbyEvent (delegate Custom|Hunger%20Loop) 5.0 true)
  (Utilities|Time|SetTimerbyEvent (delegate Custom|Needs%20Loop) 1.0 true))

(fn ConstructionScript)

(fn UpdateDebugStateText
  (Rendering|Components|TextRender|SetText (Variables|Default|GetCurrentState) (Utilities|Text|FormatText "{State} 
Health {Health} 
Backpack: {current} / {max}" (Utilities|Text|ToText(String) (Utilities|String|EnumtoString (Variables|Default|GetState))) (Variables|Stats|GetHealth) (Variables|Raid|GetFoundStuff) (Variables|Raid|GetBackpack%20Size))))

(fn FindNewTarget
  (bind _enemies (Variables|Combat|GetEnemies))
  (CallFunction|CheckAutoRaid)
  (if (Variables|Raid|GetisInRaidMode)
    ;[1 1 1] Go to city location
    (Variables|Movement|SetTarget%20Location (.RandomLocation (Class|NavigationSystem|GetRandomPointinNavigableRadius (Math|Vector|MakeVector 0.0 5e+03 0.0) (Variables|Movement|GetRadius%20For%20Target%20Search))))
    (Variables|Default|SetState "NewEnumerator1")
    (else
      ;[1 1 1] Enemy Spotted - attack
      (if (== (Utilities|Array|Length _enemies) 0)
        ;[1 1 1] No enemies - Patrol
        (Variables|Movement|SetTarget%20Location (.RandomLocation (Class|NavigationSystem|GetRandomPointinNavigableRadius (Math|Vector|MakeVector 0.0 0.0 0.0) (Variables|Movement|GetRadius%20For%20Target%20Search))))
        (Variables|Default|SetState "NewEnumerator1")
        (else
          (Variables|Combat|SetTarget%20To%20Attack (Utilities|Array|Get(acopy) _enemies))
          (Variables|Default|SetState "NewEnumerator2"))))))

(fn MakeRandomColor
  (Utilities|FlowControl|Sequence
    (:then_0
      ;[1 1 1] Skin
      (switch int (Math|Random|RandomIntegerinRange 0 5)
        (:Default
          (LocalVariables|SetSkinColor "(R=1.000000,G=0.706511,B=0.682292,A=1.000000)"))
        (:0
          (LocalVariables|SetSkinColor "(R=1.000000,G=0.706511,B=0.682292,A=1.000000)"))
        (:1
          (LocalVariables|SetSkinColor "(R=1.000000,G=0.928451,B=0.601163,A=1.000000)"))
        (:2
          (LocalVariables|SetSkinColor "(R=0.364583,G=0.237969,B=0.163590,A=1.000000)"))
        (:3
          (LocalVariables|SetSkinColor "(R=0.130208,G=0.084989,B=0.058425,A=1.000000)"))
        (:4
          (LocalVariables|SetSkinColor "(R=0.802083,G=0.533487,B=0.517521,A=1.000000)"))
        (:5
          (LocalVariables|SetSkinColor "(R=0.911458,G=0.618524,B=0.517586,A=1.000000)"))))
    (:then_1
      ;[1 1 1] Eyes
      (switch int (Math|Random|RandomIntegerinRange 0 5)
        (:Default
          (LocalVariables|SetEyesColor "(R=0.038389,G=0.363316,B=1.000000,A=1.000000)"))
        (:0
          (LocalVariables|SetEyesColor "(R=0.458333,G=0.223973,B=0.054905,A=1.000000)"))
        (:1
          (LocalVariables|SetEyesColor "(R=0.000000,G=0.144330,B=1.000000,A=1.000000)"))
        (:2
          (LocalVariables|SetEyesColor "(R=0.127718,G=0.364583,B=0.171537,A=1.000000)"))
        (:3
          (LocalVariables|SetEyesColor "(R=0.028954,G=0.130208,B=0.044175,A=1.000000)"))
        (:4
          (LocalVariables|SetEyesColor "(R=0.477431,G=0.556906,B=0.572917,A=1.000000)"))
        (:5
          (LocalVariables|SetEyesColor "(R=0.229167,G=0.100863,B=0.040582,A=1.000000)"))))
    (:then_2
      (Rendering|Material|SetVectorParameterValueonMaterials (Variables|Default|GetBody) "Color" (Math|Conversions|ToVector(LinearColor) (LocalVariables|GetSkinColor)))
      (Rendering|Components|Light|SetLightColor (Variables|Default|GetPointLight1) (LocalVariables|GetEyesColor) true))))

(fn Heal
  (bind _camp (CallFunction|GetCamp))
  (if (not (Variables|Combat|GetbIsInCombat))
    (if (< (Variables|Stats|GetHealth) (Variables|Stats|GetMaxHealth))
      (if (> (Variables|/Game/BP_Camp.BP_Camp_C|GetMaterials _camp) 0.1)
        (Variables|/Game/BP_Camp.BP_Camp_C|SetMaterials _camp (- (Variables|/Game/BP_Camp.BP_Camp_C|GetMaterials _camp) 0.1))
        (Variables|Stats|SetHealth (Math|Float|Clamp(Float) (+ (Variables|Stats|GetHealth) (Math|Random|RandomFloatinRange 1e+01 25.0)) (Variables|Stats|GetHealth) (Variables|Stats|GetMaxHealth)))))))

(fn UnloadResourcesatCamp
  ;[1 1 1] Unload resources back in camp
  (if (> (Variables|Raid|GetFoundStuff) 0.0)
    (Default|UnloadResources (CallFunction|GetCamp) (Variables|Raid|GetFoundStuff))
    (Variables|Raid|SetFoundStuff 0.0))
  (Variables|Default|SetState "NewEnumerator0"))

(fn LookforResourcesinRaid
  (if (>= (Variables|Raid|GetFoundStuff) (Variables|Raid|GetBackpack%20Size))
    (CallFunction|CallBackfromRaid)
    (else
      (bind _asbp_raid_building (Utilities|Casting|CastToBP_RaidBuilding (Utilities|Array|Get(acopy) (Collision|GetOverlappingActors "/Game/BP_RaidBuilding.BP_RaidBuilding_C" :!class /Script/Engine.Actor)))
        (:then
          (if (Variables|/Game/BP_RaidBuilding.BP_RaidBuilding_C|GetisLooted _asbp_raid_building)
            (Variables|Default|SetState "NewEnumerator0")
            (else
              (Variables|/Game/BP_RaidBuilding.BP_RaidBuilding_C|SetisLooted _asbp_raid_building true)
              (Variables|Raid|SetFoundStuff (+ (Variables|Raid|GetFoundStuff) (Math|Random|RandomFloatinRange 3.0 1e+01)))
              (Variables|Default|SetState "NewEnumerator0"))))
        (:CastFailed
          (Variables|Default|SetState "NewEnumerator0"))))))

(fn MovingLogic
  (AI|Navigation|SimpleMovetoLocation (AI|GetAIController self) (Variables|Movement|GetTarget%20Location))
  (Utilities|IsValid (Variables|Combat|GetTarget%20To%20Attack)
    (:Is%20Valid
      (Variables|Default|SetState "NewEnumerator2"))
    (:Is%20Not%20Valid
      (if (<= (Math|Vector|VectorLength (- (Transformation|GetActorLocation) (Variables|Movement|GetTarget%20Location))) 1.5e+02)
        (if (Variables|Raid|GetisInRaidMode)
          (Raid|LookforResourcesinRaid)
          (else
            (Raid|UnloadResourcesatCamp)))))))

(fn IsCombatEndedandNoEnemiesLeft?
  (bind _enemies (Variables|Combat|GetEnemies))
  (CallFunction|CheckEnemyValidity)
  (if (== (Utilities|Array|Length _enemies) 0)
    (Variables|Default|SetState "NewEnumerator0")
    (CallFunction|CombatEnded)
    (else
      (Variables|Combat|SetTarget%20To%20Attack (Utilities|Array|Get(acopy) _enemies)))))

(fn AttackTarget
  (bind _target_to_attack (Variables|Combat|GetTarget%20To%20Attack))
  (bind _returnvalue (Transformation|GetActorLocation _target_to_attack))
  (Transformation|SetActorRotation (Math|Rotator|MakeRotator 0.0 0.0 (.yaw (Math|Rotator|FindLookatRotation (Transformation|GetActorLocation) _returnvalue))))
  (Variables|Movement|SetTarget%20Location _returnvalue)
  (CallFunction|PlayAttackAnimation)
  (Class|BPIDamageable|TakeDamage(Message) (Variables|Combat|GetTarget%20To%20Attack) (Variables|Combat|GetDamage)))

(fn OnTakeDamage
  (params (Damage :type Float%20%28single-precision%29))
  (bind _output_get (Variables|Stats|SetHealth (Math|Float|Clamp(Float) (- (Variables|Stats|GetHealth) Damage) 0.0 (Variables|Stats|GetHealth))))
  (if (== _output_get 0.0)
    (Effects|SpawnEmitteratLocation "/Game/StarterContent/Particles/P_Explosion.P_Explosion" (Transformation|GetActorLocation))
    (Actor|DestroyActor)))

(fn CheckEnemyValidity
  (bind _enemies (Variables|Combat|GetEnemies))
  (for _array_element _enemies
    (Utilities|IsValid _array_element
      (:Is%20Not%20Valid
        (Utilities|Array|RemoveItem _enemies _array_element)))))

(fn CheckAutoRaid
  (bind _outactors (Actor|GetAllActorsOfClass "BP_Survivor_C"))
  (if (< (Variables|/Game/BP_Camp.BP_Camp_C|GetSurvivors%20In%20Raid (CallFunction|GetCamp)) (/ (Math|Conversions|ToFloat(Integer) (Utilities|Array|Length _outactors)) (Variables|Raid|GetAutoRaidPercent)))
    (if (== (Math|Random|RandomIntegerinRange 0 5) 5)
      (CallFunction|GotoRaid)
      (Class|NavMovementComponent|StopActiveMovement (Variables|Character|GetCharacterMovement))
      (CallFunction|FindNewTarget))
    (elif (Variables|Raid|GetisInRaidMode)
      (CallFunction|CallBackfromRaid))))

(fn UpdateDebugData
  (bind _currentstate (Variables|Default|GetCurrentState))
  ;[1 1 1] Debug State
  (Transformation|SetWorldRotation _currentstate (Math|Rotator|FindLookatRotation (Transformation|GetWorldLocation _currentstate) (Camera|GetCameraLocation (Game|GetPlayerCameraManager 0))) false false)
  (CallFunction|UpdateDebugStateText))

(fn Eat
  (bind _camp (CallFunction|GetCamp))
  (if (> (Variables|Stats|GetHunger) 3.0)
    (if (> (Variables|/Game/BP_Camp.BP_Camp_C|GetFood _camp) 0.1)
      (Variables|Stats|SetHunger (- (Variables|Stats|GetHunger) 1.0))
      (Variables|/Game/BP_Camp.BP_Camp_C|SetFood _camp (- (Variables|/Game/BP_Camp.BP_Camp_C|GetFood _camp) 0.1))
      (Rendering|Components|TextRender|SetTextRenderColor (Variables|Default|GetCurrentState) (Math|Color|MakeColor 255 255 255 255))
      (else
        (Variables|Stats|SetHealth (- (Variables|Stats|GetHealth) (Variables|Stats|GetHunger)))
        (Rendering|Components|TextRender|SetTextRenderColor (Variables|Default|GetCurrentState) (Math|Color|MakeColor 0 0 255 255))))))