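; BP_WaveSpawner is a spawner actor that periodically adds batches of BP_Zombie to the world.
; BeginPlay starts a looping timer on SpawnTimer that fires the Spawn event.
; Spawn skips the batch if CountZombies exceeds MaxAmountInWorld, otherwise it loops a small random number of times, spawning at the Arrow's transform with a Delay after each spawn.
; The cap is checked once per batch, so the population can overshoot it.
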(event Custom|Spawn
  (bind _amount_of_zombies (CallFunction|CountZombies))
  (if (not (> _amount_of_zombies (Variables|Default|GetMaxAmountInWorld)))
    (for _index (range 0 (Math|Random|RandomIntegerinRange 0 4))
      (Game|SpawnActorfromClass "/Game/BP_Zombie.BP_Zombie_C" (Transformation|GetWorldTransform (Variables|Default|GetArrow)) "AlwaysSpawn" 0 0)
      (Utilities|FlowControl|Delay 1.0))))

(event EventBeginPlay
  (Utilities|Time|SetTimerbyEvent (delegate Custom|Spawn) (Variables|Default|GetSpawnTimer) true))

(event Collision|EventActorBeginOverlap
  (params (OtherActor :type Actor%20Object%20Reference)))

(event EventTick
  (params (DeltaSeconds :type Float%20%28single-precision%29)))

(fn ConstructionScript)