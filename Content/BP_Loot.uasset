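; BP_Loot is a pickup that delivers a random amount of resources to the camp and then destroys itself.
; It is collected by clicking its cube or by a BP_Survivor overlapping it, with a click raising the maximum yield by a bonus multiplier.
; A looping PulseLight timeline drives a Light material parameter on the cube so it pulses.
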(event OnClicked(Cube)
  (params (TouchedComponent :type Primitive%20Component%20Object%20Reference) (ButtonPressed :type Key%20Structure))
  ;[0.04065 0.3368 1] Get Loot by click or by survivor
  (Variables|Default|SetMaxLootAmount (* (Variables|Default|GetMaxLootAmount) 1.2))
  (CallFunction|GetLoot))

(event OnComponentBeginOverlap(Cube)
  (params (OverlappedComponent :type Primitive%20Component%20Object%20Reference) (OtherActor :type Actor%20Object%20Reference) (OtherComp :type Primitive%20Component%20Object%20Reference) (OtherBodyIndex :type Integer) (bFromSweep :type Boolean) (SweepResult :type Hit%20Result%20Structure%20%28by%20ref%29))
  ;[0.04065 0.3368 1] Get Loot by click or by survivor
  (Utilities|Casting|CastToBP_Survivor OtherActor)
  (CallFunction|GetLoot))

(event Custom|Loop%20Timeline
  (bind _light (Timeline|Pulse%20Light PlayFromStart)
    (:Update
      (Rendering|Material|SetScalarParameterValueonMaterials (Variables|Default|GetCube) "Light" _light))
    (:Finished
      (CallFunction|LoopTimeline))))

(event Custom|Set%20Max%20Loot%20Amount
  (params (Max%20Loot%20Amount :type Float%20%28single-precision%29))
  (Variables|Default|SetMaxLootAmount Max%20Loot%20Amount))

(event Custom|Get%20Loot
  (bind _maxlootamount (Variables|Default|GetMaxLootAmount))
  (Actor|DestroyActor)
  (Default|UnloadResources (CallFunction|GetCamp) (Math|Random|RandomFloatinRange (/ _maxlootamount 2.0) _maxlootamount)))

(event EventBeginPlay
  (bind _light (Timeline|Pulse%20Light Play)
    (:Update
      (Rendering|Material|SetScalarParameterValueonMaterials (Variables|Default|GetCube) "Light" _light))
    (:Finished
      (CallFunction|LoopTimeline))))

(fn ConstructionScript)