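; BP_Decoration is a destructible prop that appears as a random camp fire, lamp or barricade.
; On BeginPlay it unhides one of the three components and its children at random.
; TakeDamage subtracts from Health, clamped between zero and its current value, so negative damage cannot heal.
; At zero Health it spawns an explosion emitter at its location and destroys itself.
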(event EventBeginPlay
  (switch int (Math|Random|RandomIntegerinRange 0 2)
    (:0
      (Development|SetHiddeninGame (Variables|Default|GetCampFire) false true))
    (:1
      (Development|SetHiddeninGame (Variables|Default|GetLamp) false true))
    (:2
      (Development|SetHiddeninGame (Variables|Default|GetBarricade) false true))))

(event Collision|EventActorBeginOverlap
  (params (OtherActor :type Actor%20Object%20Reference)))

(event EventTakeDamage
  (params (Damage :type Float%20%28single-precision%29))
  (bind _output_get (Variables|Default|SetHealth (Math|Float|Clamp(Float) (- (Variables|Default|GetHealth) Damage) 0.0 (Variables|Default|GetHealth))))
  (if (== _output_get 0.0)
    (Effects|SpawnEmitteratLocation "/Game/StarterContent/Particles/P_Explosion.P_Explosion" (Transformation|GetActorLocation))
    (Actor|DestroyActor)))

(event EventTick
  (params (DeltaSeconds :type Float%20%28single-precision%29)))

(fn ConstructionScript)