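; Player controller that provides debug-style hotkeys for game speed and trap placement under the cursor.
; The number keys 0 to 3 pass matching speed values to SetGameSpeed.
; The T key traces under the cursor against WorldStatic objects, then spawns a scaled-down BP_Trap at the hit point only if a small capsule overlap finds no WorldDynamic actors there.
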(event EventBeginPlay)

(event EventTick
  (params (DeltaSeconds :type Float%20%28single-precision%29)))

(event Input|KeyboardEvents|1
  (params (Key :type Key%20Structure))
  ;[1 1 1] Game Speed Control
  (:Pressed
    (CallFunction|SetGameSpeed 1.0)))

(event Input|KeyboardEvents|2
  (params (Key :type Key%20Structure))
  ;[1 1 1] Game Speed Control
  (:Pressed
    (CallFunction|SetGameSpeed 2.0)))

(event Input|KeyboardEvents|3
  (params (Key :type Key%20Structure))
  ;[1 1 1] Game Speed Control
  (:Pressed
    (CallFunction|SetGameSpeed 3.0)))

(event Input|KeyboardEvents|0
  (params (Key :type Key%20Structure))
  ;[1 1 1] Game Speed Control
  (:Pressed
    (CallFunction|SetGameSpeed 0.0)))

(event Input|KeyboardEvents|T
  (params (Key :type Key%20Structure))
  (bind _array (Utilities|Array|MakeArray "ObjectTypeQuery1"))
  (bind (_hitresult _returnvalue) (Class|PlayerController|GetHitResultUnderCursorforObjects _array true))
  (bind _location (Collision|BreakHitResult _hitresult))
  (:Pressed
    (if _returnvalue
      (bind _returnvalue_2 (Collision|CapsuleOverlapActors _location 1e+01 0.0 (Utilities|Array|MakeArray "ObjectTypeQuery2") 0))
      (if (not _returnvalue_2)
        (Game|SpawnActorfromClass "/Game/BP_Trap.BP_Trap_C" (Math|Transform|MakeTransform _location "0, 0, 0" "0.200000,0.200000,0.200000") "Undefined" 0 0)))))

(fn ConstructionScript)